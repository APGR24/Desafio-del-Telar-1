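; Hilado (spinning) is an interactable that shows a button prompt when the player is near and plays Rueca (spinning wheel) on Agarrar (grab) input.
; Entering the Box creates a new Boton widget, shown only for the player character and removed when that character leaves.
; Overlaps from any actor toggle the Cerca4 proximity flag, but the input plays Rueca without checking it.
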(event OnComponentBeginOverlap(Box)
  (params (OverlappedComponent :type Primitive%20Component%20Object%20Reference) (OtherActor :type Actor%20Object%20Reference) (OtherComp :type Primitive%20Component%20Object%20Reference) (OtherBodyIndex :type Integer) (bFromSweep :type Boolean) (SweepResult :type Hit%20Result%20Structure%20%28by%20ref%29))
  (Utilities|FlowControl|Sequence
    (:then_0
      (bind _returnvalue (UserInterface|CreateWidget "/Game/Widgets/Boton.Boton_C"))
      (Variables|Default|SetInteraccion%204 _returnvalue))
    (:then_1
      (Variables|Default|SetCerca%204 true)
      (if (== OtherActor (Game|GetPlayerCharacter 0))
        (UserInterface|Viewport|AddtoViewport (Variables|Default|GetInteraccion%204) 0)))))

(event OnComponentEndOverlap(Box)
  (params (OverlappedComponent :type Primitive%20Component%20Object%20Reference) (OtherActor :type Actor%20Object%20Reference) (OtherComp :type Primitive%20Component%20Object%20Reference) (OtherBodyIndex :type Integer))
  (Variables|Default|SetCerca%204 false)
  (if (== (Game|GetPlayerCharacter 0) OtherActor)
    (Widget|RemovefromParent (Variables|Default|GetInteraccion%204))))

(event Input|ActionEvents|InputActionAgarrar
  (params (Key :type Key%20Structure :default "None"))
  (:Pressed
    (Timeline|Rueca Play)))

(fn ConstructionScript)
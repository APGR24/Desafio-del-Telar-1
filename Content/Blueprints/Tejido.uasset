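; Tejido is an actor with a Box trigger that shows an interaction widget when the player is nearby.
; On BeginPlay it creates a Boton_Herramientas widget and stores it as Interaccion7.
; Box overlaps add or remove that widget from the viewport for player character 0 only.
; The Cerca7 proximity flag toggles for any overlapping actor and is not read in this graph.
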(event OnComponentBeginOverlap(Box)
  (params (OverlappedComponent :type Primitive%20Component%20Object%20Reference) (OtherActor :type Actor%20Object%20Reference) (OtherComp :type Primitive%20Component%20Object%20Reference) (OtherBodyIndex :type Integer) (bFromSweep :type Boolean) (SweepResult :type Hit%20Result%20Structure%20%28by%20ref%29))
  (Variables|Default|SetCerca%207 true)
  (if (== OtherActor (Game|GetPlayerCharacter 0))
    (UserInterface|Viewport|AddtoViewport (Variables|Default|GetInteraccion%207) 0)))

(event OnComponentEndOverlap(Box)
  (params (OverlappedComponent :type Primitive%20Component%20Object%20Reference) (OtherActor :type Actor%20Object%20Reference) (OtherComp :type Primitive%20Component%20Object%20Reference) (OtherBodyIndex :type Integer))
  (Variables|Default|SetCerca%207 false)
  (if (== (Game|GetPlayerCharacter 0) OtherActor)
    (Widget|RemovefromParent (Variables|Default|GetInteraccion%207))))

(event EventBeginPlay
  (bind _returnvalue (UserInterface|CreateWidget "/Game/Widgets/Boton_Herramientas.Boton_Herramientas_C"))
  (Variables|Default|SetInteraccion%207 _returnvalue))

(fn ConstructionScript)